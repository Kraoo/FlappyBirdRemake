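; Player character for a Flappy Bird-style game, moved by physics forces on its Capsule.
; Pressing Jumping zeroes the capsule's velocity, then applies an upward force for the flap.
; While rising, Tick adds a delta-time-scaled downforce that is much weaker while the Jumping axis is held, giving variable jump height.
; No extra force is applied while falling.
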(event `self.ReceiveTick`
  (params (DeltaSeconds :type "Float (single-precision)"))
  (bind _returnvalue (`PrimitiveComponent.GetPhysicsLinearVelocity` (`self.Capsule`) "None"))
  (if (> (.z _returnvalue) 0.0)
    (if (== (`self.GetInputAxisValue`) 1.0)
      (set `self.Downforce` (* -3000.0 DeltaSeconds))
      (else
        (set `self.Downforce` (* -35000.0 DeltaSeconds))))
    (`PrimitiveComponent.AddForce` (`self.Capsule`) (`KismetMathLibrary.MakeVector` 0.0 0.0 (`self.Downforce`)) "None" false)))

(event `InputAction|Jumping`
  (params (Key :type "Key Structure"))
  (:`Pressed`
    (`PrimitiveComponent.SetPhysicsLinearVelocity` (`self.Capsule`) (0.0 0.0 0.0) false "None")
    (`PrimitiveComponent.AddForce` (`self.Capsule`) (0.0 0.0 26000.0) "None" false)))

(event `InputAxis|Jumping`
  (params (AxisValue :type "Float (single-precision)")))

(fn `UserConstructionScript`)